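; BP_CubeSpawner is an actor that builds a grid of scaled BP_CubeActor instances at BeginPlay, starting from its root location.
; Each cube's LeftLocation places the next cube in the row, while FrontLocation places the first cube of the following row.
; A DoOnce captures the initial front position, then RedrawCubes calls itself recursively, advancing CubeCount until it exceeds Column.
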(event Custom|RedrawCubes
  (for _index (range 0 (Variables|Default|GetRow))
    (bind _returnvalue (Game|SpawnActorfromClass "/Game/Blueprints/Levels/BP_CubeActor.BP_CubeActor_C" (Math|Transform|MakeTransform (Variables|Default|GetNextLocation) "0, 0, 0" (Variables|Default|GetCubeScale)) "AlwaysSpawn" 0 0))
    (Variables|Default|SetNextLocation (Variables|/Game/Blueprints/Levels/BP_CubeActor.BP_CubeActor_C|GetLeftLocation _returnvalue))
    (Utilities|FlowControl|DoOnce false
      (:Completed
        (Variables|Default|SetFrontLocation (Variables|/Game/Blueprints/Levels/BP_CubeActor.BP_CubeActor_C|GetFrontLocation _returnvalue)))))
  (bind _returnvalue_2 (Game|SpawnActorfromClass "/Game/Blueprints/Levels/BP_CubeActor.BP_CubeActor_C" (Math|Transform|MakeTransform (Variables|Default|GetFrontLocation) "0, 0, 0" (Variables|Default|GetCubeScale)) "AlwaysSpawn" 0 0))
  (Variables|Default|SetNextLocation (Variables|/Game/Blueprints/Levels/BP_CubeActor.BP_CubeActor_C|GetLeftLocation _returnvalue_2))
  (Variables|Default|SetFrontLocation (Variables|/Game/Blueprints/Levels/BP_CubeActor.BP_CubeActor_C|GetFrontLocation _returnvalue_2))
  (if (<= (Variables|Default|GetCubeCount) (Variables|Default|GetColumn))
    (Variables|Default|SetCubeCount (+ (Variables|Default|GetCubeCount) 1))
    (CallFunction|RedrawCubes)))

(event EventBeginPlay
  (Variables|Default|SetNextLocation (Transformation|GetWorldLocation (Variables|Default|GetDefaultSceneRoot)))
  (for _index (range 0 (Variables|Default|GetRow))
    (bind _returnvalue (Game|SpawnActorfromClass "/Game/Blueprints/Levels/BP_CubeActor.BP_CubeActor_C" (Math|Transform|MakeTransform (Variables|Default|GetNextLocation) "0, 0, 0" (Variables|Default|GetCubeScale)) "AlwaysSpawn" 0 0))
    (Variables|Default|SetNextLocation (Variables|/Game/Blueprints/Levels/BP_CubeActor.BP_CubeActor_C|GetLeftLocation _returnvalue))
    (Utilities|FlowControl|DoOnce false
      (:Completed
        (Variables|Default|SetFrontLocation (Variables|/Game/Blueprints/Levels/BP_CubeActor.BP_CubeActor_C|GetFrontLocation _returnvalue)))))
  (bind _returnvalue_2 (Game|SpawnActorfromClass "/Game/Blueprints/Levels/BP_CubeActor.BP_CubeActor_C" (Math|Transform|MakeTransform (Variables|Default|GetFrontLocation) "0, 0, 0" (Variables|Default|GetCubeScale)) "AlwaysSpawn" 0 0))
  (Variables|Default|SetNextLocation (Variables|/Game/Blueprints/Levels/BP_CubeActor.BP_CubeActor_C|GetLeftLocation _returnvalue_2))
  (Variables|Default|SetFrontLocation (Variables|/Game/Blueprints/Levels/BP_CubeActor.BP_CubeActor_C|GetFrontLocation _returnvalue_2))
  (if (<= (Variables|Default|GetCubeCount) (Variables|Default|GetColumn))
    (Variables|Default|SetCubeCount (+ (Variables|Default|GetCubeCount) 1))
    (CallFunction|RedrawCubes)))

(fn ConstructionScript)