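; BP_DisintegrateActor is a showcase actor that repeatedly dissolves and restores a mesh through a disintegration material.
; The construction script creates a dynamic instance of MI_Disintegrate, assigns the showcase mesh, and applies the dissolve texture, dissolve color and base color from its variables.
; A looping timer calls Disintegrate, where a FlipFlop alternately plays and reverses a timeline that drives the material's Amount parameter.
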(event Custom|Disintegrate
  (Utilities|FlowControl|FlipFlop
    (:A
      (bind _amount (Timeline|AnimDisintegration PlayFromStart)
        (:Update
          (Rendering|Material|SetScalarParameterValue (Variables|Default|GetMID) "Amount" _amount :!class /Script/Engine.MaterialInstanceDynamic))))
    (:B
      (Timeline|AnimDisintegration ReverseFromEnd))))

(event EventBeginPlay
  (Utilities|Time|SetTimerbyFunctionName 0 "Disintegrate" 2.0 true))

(fn ConstructionScript
  (bind _returnvalue (Rendering|Material|CreateDynamicMaterialInstance (Variables|Default|GetStaticMesh) 0 "/Game/Materials/Base/MI_Disintegrate.MI_Disintegrate" :!class /Script/Engine.PrimitiveComponent))
  (Variables|Default|SetMID _returnvalue)
  (Components|StaticMesh|SetStaticMesh (Variables|Default|GetStaticMesh) (Variables|Default|GetShowcaseMesh))
  (Rendering|Material|SetTextureParameterValue (Variables|Default|GetMID) "ColorTexture" (Variables|Default|GetDissolveTexture))
  (Rendering|Material|SetVectorParameterValue (Variables|Default|GetMID) "DissolveColor" (Variables|Default|GetDissolveColor) :!class /Script/Engine.MaterialInstanceDynamic)
  (Rendering|Material|SetVectorParameterValue (Variables|Default|GetMID) "BaseColor" (Variables|Default|GetMeshColor) :!class /Script/Engine.MaterialInstanceDynamic))