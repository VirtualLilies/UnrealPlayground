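; Base weapon Blueprint that provides shared firing effects and aim calculation.
; FireWeapon plays the fire sound and attaches muzzle flash and trail emitters at the Muzzle socket, while StopFireWeapon is empty.
; CalculateShootInfo traces 100 m from the camera given via SetCamera and returns a muzzle transform aimed at the hit or trace end, correcting camera-to-muzzle offset.
; The trace draws debug lines, and nothing here calls that function.
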(event Custom|FireWeapon
  (CallFunction|SpawnShootEffects))

(event Custom|StopFireWeapon)

(fn ConstructionScript)

(fn CalculateShootInfo
  (bind _playercamera (Variables|Default|GetPlayerCamera))
  (bind _weaponmesh (Variables|Default|GetWeaponMesh))
  (bind _returnvalue (Transformation|GetWorldLocation _playercamera))
  (bind _returnvalue_2 (Math|Vector|GetForwardVector _playercamera))
  (bind _returnvalue_3 (Transformation|GetSocketLocation _weaponmesh "Muzzle"))
  (bind _returnvalue_4 (* _returnvalue_2 1e+04))
  (bind _returnvalue_5 (+ _returnvalue _returnvalue_4))
  (bind (_outhit _returnvalue_6) (Collision|LineTraceByChannel _returnvalue _returnvalue_5 "TraceTypeQuery3" false 0 "ForDuration"))
  (if _returnvalue_6
    (return (Math|Transform|MakeTransform _returnvalue_3 (Math|Rotator|FindLookatRotation _returnvalue_3 (.Location (Collision|BreakHitResult _outhit)))))
    (else
      (return (Math|Transform|MakeTransform _returnvalue_3 (Math|Rotator|FindLookatRotation _returnvalue_3 _returnvalue_5))))))

(fn SetCamera
  (params (Camera :type Camera%20Component%20Object%20Reference))
  (Variables|Default|SetPlayerCamera Camera))

(fn SpawnShootEffects
  (Audio|PlaySoundatLocation (Variables|SFX|GetFireSFX) (Transformation|GetActorLocation))
  (Effects|SpawnEmitterAttached (Variables|VFX|GetMuzzleFlash) (Variables|Default|GetWeaponMesh) "Muzzle" "0, 0, 0" "0, 0, 0" "1.000000,1.000000,1.000000" "SnapToTarget")
  (Effects|SpawnEmitterAttached "/Game/Particles/P_Trail.P_Trail" (Variables|Default|GetWeaponMesh) "Muzzle" "0, 0, 0" "0.000000, 0, 0" "1.000000,1.000000,1.000000" "SnapToTarget") ; Spawned due to the ShooterTemplate particle being not suitable for this system
)