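; Assault rifle weapon Blueprint that adds fully automatic fire to its parent weapon's firing logic.
; FireWeapon fires once immediately, then starts a looping timer at the FireRate interval that calls the parent's FireWeapon while the firing flag is set.
; StopFireWeapon clears that flag and invalidates the timer to end the burst.
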(event Custom|AutoFire
  (if (Variables|Default|GetIsFiring)
    (|CallParentFunction)))

(event EventFireWeapon
  (Variables|Default|SetIsFiring true)
  (CallFunction|AutoFire)
  (bind _returnvalue (Utilities|Time|SetTimerbyEvent (delegate Custom|AutoFire) (Variables|Default|GetFireRate) true))
  (Variables|Default|SetFireTimer _returnvalue))

(event EventStopFireWeapon
  (Variables|Default|SetIsFiring false)
  (Utilities|Time|ClearandInvalidateTimerbyHandle (Variables|Default|GetFireTimer)))

(fn ConstructionScript
  (|CallParentFunction))