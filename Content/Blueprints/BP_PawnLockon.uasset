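; Player pawn with a toggled lock-on camera for BP_LockonEnemy targets, plus an F key that calls SeekPlayer on those enemies.
; Target input picks the nearest enemy within range that passes a line-trace visibility check, notifies it and toggles a gate fed by LoopingTimeline updates.
; The gate drives yaw-only interpolation toward the target, while lock blocks manual turning, dampens pitch input and enables controller-yaw rotation.
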(event Input|ActionEvents|InputActionTarget
  (params (Key :type Key%20Structure))
  (:Pressed
    (Variables|Lockon|SetClosestTargetDistance (Variables|Lockon|GetMinDistanceToEnable))
    (if (Variables|Lockon|GetIsTargetLocked)
      (Variables|Lockon|SetIsTargetLocked false)
      (Class|BPILockon|TargetLockon(Message) (Variables|Lockon|GetNearestTarget) :!label _label)
      (Utilities|FlowControl|Gate true) ; enters at Toggle
      (else
        (bind _outactors (Actor|GetAllActorsOfClass "/Game/Blueprints/AI/BP_LockonEnemy.BP_LockonEnemy_C"))
        (for _array_element _outactors
          (bind _outhit (Collision|LineTraceForObjects (Transformation|GetActorLocation) (Transformation|GetActorLocation _array_element) (Utilities|Array|MakeArray "ObjectTypeQuery1" "ObjectTypeQuery2" "ObjectTypeQuery3") false 0 "ForDuration"))
          (if (== _array_element (.HitActor (Collision|BreakHitResult _outhit)))
            (bind _distancefromplayer (Default|DistancefromPlayerCheck _array_element))
            (Math|Float|CompareFloat _distancefromplayer (Variables|Lockon|GetClosestTargetDistance)
              (:<
                (Variables|Lockon|SetClosestTargetDistance _distancefromplayer)
                (Variables|Lockon|SetNearestTarget _array_element)))))
        (if (< (Variables|Lockon|GetClosestTargetDistance) (Variables|Lockon|GetMinDistanceToEnable))
          (Variables|Lockon|SetIsTargetLocked true)
          (goto _label))))))

(event Input|AxisEvents|InputAxisLookUp
  (params (AxisValue :type Float%20%28single-precision%29))
  (bind _istargetlocked (Variables|Lockon|GetIsTargetLocked))
  ;[0 1 0] Overrided Mouse Input
  (Pawn|Input|AddControllerPitchInput (* AxisValue (Math|Float|SelectFloat 0.2 1.0 _istargetlocked)))
  (Variables|Default|SetbUseControllerRotationYaw _istargetlocked))

(event Input|AxisEvents|InputAxisTurn
  (params (AxisValue :type Float%20%28single-precision%29))
  (bind _istargetlocked (Variables|Lockon|GetIsTargetLocked))
  ;[0 1 0] Overrided Mouse Input
  (if (not _istargetlocked)
    (Pawn|Input|AddControllerYawInput AxisValue)
    (Variables|Default|SetbUseControllerRotationYaw _istargetlocked)))

(event Input|KeyboardEvents|F
  (params (Key :type Key%20Structure))
  (:Pressed
    (bind _outactors (Actor|GetAllActorsOfClass "/Game/Blueprints/AI/BP_LockonEnemy.BP_LockonEnemy_C"))
    (Default|SeekPlayer _outactors)))

(fn ConstructionScript
  (|CallParentFunction))

(fn ChangeCameraandPlayerRotationwhenTarget
  (bind _returnvalue (Pawn|GetController))
  (bind _returnvalue_2 (Pawn|GetControlRotation _returnvalue :!class /Script/Engine.Controller))
  (bind (_roll _pitch) (Math|Rotator|BreakRotator _returnvalue_2))
  (return _returnvalue (Math|Rotator|MakeRotator _roll _pitch (.Yaw (Math|Rotator|BreakRotator (Math|Interpolation|RInterpTo _returnvalue_2 (Math|Rotator|FindLookatRotation (Transformation|GetWorldLocation (Variables|Default|GetFollowCamera)) (Transformation|GetActorLocation (Variables|Lockon|GetNearestTarget))) (Utilities|Time|GetWorldDeltaSeconds) 7.0))))))