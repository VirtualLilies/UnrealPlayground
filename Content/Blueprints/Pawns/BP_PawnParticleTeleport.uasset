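; Character Blueprint that provides two particle "teleport" dashes, hiding the mesh behind an opacity material and overlapping WorldDynamic objects during the effect.
; Holding E launches along the camera and boosts walk speed until release; Q launches along TeleportVector's yaw for a timed duration, with a looping timer for repeated bursts.
; Both spawn burst and attached emitters, passing self as an actor instance parameter for vertex/surface sampling.
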(event Custom|MultipleParticleSpawn
  ;[0 0.5 1] Manage multi-effect logic
  (if (or (== (Variables|Default|GetCurrentParticleCount) (Variables|Teleport|GetMaxParticleCount)) (not (Variables|Default|GetIsEffectOn)))
    (Utilities|Time|ClearandInvalidateTimerbyHandle (Variables|Default|GetParticleTimer))
    (else
      (bind _returnvalue (Effects|SpawnEmitteratLocation "/Game/Particles/P_FirstEffect.P_FirstEffect" (Transformation|GetActorLocation)))
      (Variables|/Script/Engine.ParticleSystemComponent|SetInstanceParameters _returnvalue (Utilities|Array|MakeArray (Utilities|Struct|MakeParticleSysParam "VertSurfaceActor" "PSPT_Actor" 0.0 0.0 "0, 0, 0" "0, 0, 0" "(B=0,G=0,R=0,A=0)" self)))
      (Math|Integer|IncrementInt (Variables|Default|GetCurrentParticleCount)))))

(event Custom|ClearSingleTeleport
  (bind _mesh (Variables|Character|GetMesh))
  ;[0 1 0] Manage single effect logic
  (Rendering|Material|SetMaterial _mesh 0 "/Game/Materials/Characters/M_UE4Man_Body.M_UE4Man_Body")
  (Rendering|Material|SetMaterial _mesh 1 "/Game/Materials/Characters/M_UE4Man_ChestLogo.M_UE4Man_ChestLogo")
  (Components|Activation|Deactivate (stale Custom|SingleJump _returnvalue_2))
  (Variables|Default|SetIsEffectOn false)
  (Collision|SetCollisionResponsetoChannel (Variables|Default|GetCapsuleComponent) "ECC_WorldDynamic" "ECR_Block")
  (Variables|/Script/Engine.CharacterMovementComponent|SetMaxWalkSpeed (Variables|Character|GetCharacterMovement) 1.5e+02))

(event Custom|SingleJump
  (bind _mesh (Variables|Character|GetMesh))
  ;[0 1 0] Manage single effect logic
  (Character|LaunchCharacter (* (Math|Vector|GetForwardVector (Variables|Default|GetFollowCamera)) (Variables|Teleport|GetSingleTeleportDashMultiplier)) true true)
  (if (not (Variables|Default|GetIsEffectOn))
    (Variables|Default|SetIsEffectOn true)
    (Collision|SetCollisionResponsetoChannel (Variables|Default|GetCapsuleComponent) "ECC_WorldDynamic" "ECR_Overlap")
    (Rendering|Material|SetMaterial _mesh 0 "/Game/Materials/VFX/M_Opacity.M_Opacity")
    (Rendering|Material|SetMaterial _mesh 1 "/Game/Materials/VFX/M_Opacity.M_Opacity")
    (bind _returnvalue (Effects|SpawnEmitteratLocation "/Game/Particles/P_FirstEffect.P_FirstEffect" (Transformation|GetActorLocation)))
    (Variables|/Script/Engine.ParticleSystemComponent|SetInstanceParameters _returnvalue (Utilities|Array|MakeArray (Utilities|Struct|MakeParticleSysParam "VertSurfaceActor" "PSPT_Actor" 0.0 0.0 "0, 0, 0" "0, 0, 0" "(B=0,G=0,R=0,A=0)" self)))
    (bind _returnvalue_2 (Effects|SpawnEmitterAttached "/Game/Particles/P_SecondEffect.P_SecondEffect" (Variables|Default|GetCapsuleComponent) "None"))
    (Variables|/Script/Engine.ParticleSystemComponent|SetInstanceParameters _returnvalue_2 (Utilities|Array|MakeArray (Utilities|Struct|MakeParticleSysParam "VertSurfaceActor2" "PSPT_Actor" 0.0 0.0 "0, 0, 0" "0, 0, 0" "(B=0,G=0,R=0,A=0)" self)))
    (Variables|/Script/Engine.CharacterMovementComponent|SetMaxWalkSpeed (Variables|Character|GetCharacterMovement) 8e+02)))

(event Custom|MultipleJump
  (bind _mesh (Variables|Character|GetMesh))
  (bind _mesh_2 (Variables|Character|GetMesh))
  ;[0 0.5 1] Manage multi-effect logic
  (Character|LaunchCharacter (* (Math|Rotator|GetRotationXVector (Math|Rotator|MakeRotator 0.0 0.0 (.Yaw (Math|Rotator|BreakRotator (Transformation|GetWorldRotation (Variables|Default|GetTeleportVector)))))) (Variables|Teleport|GetJumpTeleportMultiplier)) false true)
  (Variables|Default|SetCurrentParticleCount 0)
  (if (not (Variables|Default|GetIsEffectOn))
    (Variables|Default|SetIsEffectOn true)
    (Rendering|Material|SetMaterial _mesh 0 "/Game/Materials/VFX/M_Opacity.M_Opacity")
    (Rendering|Material|SetMaterial _mesh 1 "/Game/Materials/VFX/M_Opacity.M_Opacity")
    (Collision|SetCollisionResponsetoChannel (Variables|Default|GetCapsuleComponent) "ECC_WorldDynamic" "ECR_Overlap")
    (bind _returnvalue (Effects|SpawnEmitteratLocation "/Game/Particles/P_FirstEffect.P_FirstEffect" (Transformation|GetActorLocation)))
    (Variables|/Script/Engine.ParticleSystemComponent|SetInstanceParameters _returnvalue (Utilities|Array|MakeArray (Utilities|Struct|MakeParticleSysParam "VertSurfaceActor" "PSPT_Actor" 0.0 0.0 "0, 0, 0" "0, 0, 0" "(B=0,G=0,R=0,A=0)" self)))
    (bind _returnvalue_2 (Utilities|Time|SetTimerbyEvent (EventDispatchers|CreateEvent :!event Custom|MultipleParticleSpawn) 0.3 true))
    (Variables|Default|SetParticleTimer _returnvalue_2)
    (bind _returnvalue_3 (Effects|SpawnEmitterAttached "/Game/Particles/P_SecondEffect.P_SecondEffect" (Variables|Default|GetCapsuleComponent) "None"))
    (Variables|/Script/Engine.ParticleSystemComponent|SetInstanceParameters _returnvalue_3 (Utilities|Array|MakeArray (Utilities|Struct|MakeParticleSysParam "VertSurfaceActor2" "PSPT_Actor" 0.0 0.0 "0, 0, 0" "0, 0, 0" "(B=0,G=0,R=0,A=0)" self)))
    (Utilities|FlowControl|Delay (Variables|Teleport|GetMultipleEffectDuration))
    (Rendering|Material|SetMaterial _mesh_2 0 "/Game/Materials/Characters/M_UE4Man_Body.M_UE4Man_Body")
    (Rendering|Material|SetMaterial _mesh_2 1 "/Game/Materials/Characters/M_UE4Man_ChestLogo.M_UE4Man_ChestLogo")
    (Components|Activation|Deactivate _returnvalue_3)
    (Variables|Default|SetIsEffectOn false)
    (Collision|SetCollisionResponsetoChannel (Variables|Default|GetCapsuleComponent) "ECC_WorldDynamic" "ECR_Block")))

(event Input|KeyboardEvents|E
  (params (Key :type Key%20Structure))
  ;[0 0.5 1] Key Binding
  (:Pressed
    (CallFunction|SingleJump))
  (:Released
    (CallFunction|ClearSingleTeleport)))

(event Input|KeyboardEvents|Q
  (params (Key :type Key%20Structure))
  ;[0 0.5 1] Key Binding
  (:Pressed
    (if (not (Variables|Default|GetIsEffectOn))
      (CallFunction|MultipleJump))))

(fn ConstructionScript
  (|CallParentFunction))