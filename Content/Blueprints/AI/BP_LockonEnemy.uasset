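; Enemy character that the player can lock onto, with a per-instance body color applied through dynamic materials in construction.
; Unless dead at BeginPlay, it runs a looping timer that writes its location to TargetPosition on the BP_UPGI game instance.
; TargetLockon toggles a timeline that scales the target marker and drives highlight light intensity, reversing on release.
; It also offers AI movement toward the player and a player-distance query.
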(event Custom|SeekPlayer
  ;[0 1 0] Seek Player event
  (AI|AIMoveTo self "0, 0, 0" (Game|GetPlayerCharacter 0) 1e+01 false))

(event EventTargetLockon
  ;[0 0.5 1] Trigger TargetVisual ON/OFF
  (Utilities|FlowControl|FlipFlop
    (:A
      (Development|SetHiddeninGame (Variables|Default|GetTargetVisual) false false)
      (bind (_direction _lightintensity _3dscale) (Timeline|ScaleTargetVisual PlayFromStart)
        (:Update
          (Transformation|SetRelativeScale3D (Variables|Default|GetTargetVisual) _3dscale)
          (Rendering|Components|Light|SetIntensity (Variables|Default|GetHighlight) _lightintensity))))
    (:B
      (Timeline|ScaleTargetVisual ReverseFromEnd))))

(event EventBeginPlay
  ;[1 0 0] BeginPlay
  ;[0 0.5 1] Update targets location
  (if (not (Variables|Default|GetIsDead))
    (Utilities|FlowControl|DoOnce false
      (:Completed
        (Utilities|Time|SetTimerbyFunctionName 0 "SendTargetLocation" 0.05 true)))))

(fn ConstructionScript
  (bind _bodycolor (Variables|EnemyDefaults|GetBodyColor))
  (bind _returnvalue (Rendering|Material|CreateDynamicMaterialInstance (Variables|Character|GetMesh) 0 "/Game/Materials/Characters/MI_Mannequin.MI_Mannequin" :!class /Script/Engine.PrimitiveComponent))
  (bind _output_get (LocalVariables|SetBodyMID _returnvalue))
  (Rendering|Material|SetVectorParameterValue _output_get "BodyColor" _bodycolor :!class /Script/Engine.MaterialInstanceDynamic)
  (bind _returnvalue_2 (Rendering|Material|CreateDynamicMaterialInstance (Variables|Character|GetMesh) 1 "/Game/Materials/Characters/M_UE4Man_ChestLogo.M_UE4Man_ChestLogo" :!class /Script/Engine.PrimitiveComponent))
  (Rendering|Material|SetVectorParameterValue _returnvalue_2 "BodyColor" _bodycolor :!class /Script/Engine.MaterialInstanceDynamic))

(fn SendTargetLocation
  (bind _asbp_upgi (Utilities|Casting|CastToBP_UPGI (Game|GetGameInstance)))
  (Variables|/Game/Blueprints/BP_UPGI.BP_UPGI_C|SetTargetPosition _asbp_upgi (Transformation|GetActorLocation)))

(fn DistancefromPlayerCheck
  (return (Transformation|GetDistanceTo (Game|GetPlayerCharacter 0))))